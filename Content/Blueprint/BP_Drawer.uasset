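; BP_Drawer is an interactable drawer the player can get into and out of, likely as a hiding spot.
; Interact toggles Inside, teleporting player 0 to the REFDALAM (inside) or REFLUAR (outside) reference transform with a sound.
; Each toggle also snaps the Door rotation and sets IsCanMove on the interacting actor, blocking movement while inside.
; The collision overlap only prints a debug message for the third-person character.
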(event OnComponentBeginOverlap(Collison)
  (params (OverlappedComponent :type Primitive%20Component%20Object%20Reference) (OtherActor :type Actor%20Object%20Reference) (OtherComp :type Primitive%20Component%20Object%20Reference) (OtherBodyIndex :type Integer) (bFromSweep :type Boolean) (SweepResult :type Hit%20Result%20Structure%20%28by%20ref%29))
  (Utilities|Casting|CastToBP_ThirdPersonCharacter OtherActor)
  (Development|PrintString "Hello"))

(event EventBeginPlay)

(event Collision|EventActorBeginOverlap
  (params (OtherActor :type Actor%20Object%20Reference)))

(event EventTick
  (params (DeltaSeconds :type Float%20%28single-precision%29)))

(event EventInteract
  (params (MyActor :type BP%20Third%20Person%20Character%20Object%20Reference))
  (bind _ref_luar (Variables|Default|GetREF%20LUAR))
  (bind __ref_dalam (Variables|Default|Get%20REF%20DALAM))
  (bind _returnvalue (Transformation|GetWorldTransform __ref_dalam))
  (bind _returnvalue_2 (Transformation|GetWorldTransform _ref_luar))
  (if (not (Variables|Default|GetInside))
    (Variables|Default|SetInside true)
    (Transformation|SetActorTransform (Game|GetPlayerCharacter 0) (Math|Transform|MakeTransform (.location _returnvalue) (.rotation _returnvalue) "1.000000,1.000000,1.000000"))
    (Audio|PlaySound2D "/Game/StarterContent/Audio/Collapse01.Collapse01" 0.5 1.0 0.0 0 0)
    (Transformation|SetRelativeRotation (Variables|Default|GetDoor) "0, 0, 0" false false)
    (Variables|/Game/ThirdPerson/Blueprints/BP_ThirdPersonCharacter.BP_ThirdPersonCharacter_C|SetIsCanMove MyActor false)
    (else
      (Variables|Default|SetInside false)
      (Transformation|SetActorTransform (Game|GetPlayerCharacter 0) (Math|Transform|MakeTransform (.location _returnvalue_2) (.rotation _returnvalue_2) "1.000000,1.000000,1.000000"))
      (Audio|PlaySound2D "/Game/StarterContent/Audio/Collapse01.Collapse01" 0.5 1.0 0.0 0 0)
      (Transformation|SetRelativeRotation (Variables|Default|GetDoor) "0.000000,100.000000,0.000000" false false)
      (Variables|/Game/ThirdPerson/Blueprints/BP_ThirdPersonCharacter.BP_ThirdPersonCharacter_C|SetIsCanMove MyActor true))))

(fn ConstructionScript)
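; BP_flick is a flickering light Blueprint that toggles the intensity of its Flickring light component at random intervals.
; From BeginPlay, a retriggerable delay with a random duration between Min and Max feeds a FlipFlop that alternates between NewIntensity0 and NewIntensity.
; Both branches loop back to the delay, so the flicker repeats endlessly without Tick.
; The construction script sets the light to NewIntensity as its initial state.
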(event EventBeginPlay
  (bind _flickring (Variables|Default|GetFlickring))
  (Utilities|FlowControl|RetriggerableDelay (Math|Random|RandomFloatinRange (Variables|Default|GetMin) (Variables|Default|GetMax)) :!label _label)
  (Utilities|FlowControl|FlipFlop
    (:A
      (Rendering|Components|Light|SetIntensity _flickring (Variables|Default|GetNew%20Intensity_0))
      (goto _label))
    (:B
      (Rendering|Components|Light|SetIntensity _flickring (Variables|Default|GetNew%20Intensity))
      (goto _label))))

(fn ConstructionScript
  (Rendering|Components|Light|SetIntensity (Variables|Default|GetFlickring) (Variables|Default|GetNew%20Intensity)))
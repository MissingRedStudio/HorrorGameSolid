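; BP_AI is an AI pawn that detects the player and performs a melee attack.
; Pawn sensing sets the SeeingPlayer blackboard key for pawns tagged Player, while a looping half-second timer clears it.
; AttackPlayer plays a montage, gated by an Attacking flag until completion.
; As the montage starts, a short forward sphere trace from AttackTracePoint damages any pawn it hits.
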(event OnSeePawn(PawnSensing)
  (params (Pawn :type Pawn%20Object%20Reference))
  (if (Actor|ActorHasTag Pawn "Player")
    (AI|Components|Blackboard|SetValueasBool (AI|GetBlackboard (AI|GetAIController self)) (Utilities|Name|MakeLiteralName "SeeingPlayer") true)))

(event Custom|Attack%20Player
  (bind _attack_trace_point (Variables|Default|GetAttack%20Trace%20Point))
  (bind _returnvalue (Transformation|GetWorldLocation _attack_trace_point))
  (if (not (Variables|Default|GetAttacking))
    (Variables|Default|SetAttacking true)
    (Animation|Montage|PlayMontage (Variables|Character|GetMesh) 0
      (:then
        (bind (_outhit _returnvalue_2) (Collision|SphereTraceForObjects _returnvalue (+ _returnvalue (* (Math|Vector|GetForwardVector (Transformation|GetWorldRotation _attack_trace_point)) 7e+01)) 25.0 (Utilities|Array|MakeArray "ObjectTypeQuery3") false 0 "None"))
        (if _returnvalue_2
          (Game|Damage|ApplyDamage (.HitActor (Collision|BreakHitResult _outhit)) 1e+01 0 0)))
      (:OnCompleted
        (Variables|Default|SetAttacking false)))))

(event Custom|Stop%20SeeingPlayer
  (Utilities|FlowControl|Sequence
    (:then_0
      (AI|Components|Blackboard|SetValueasBool (AI|GetBlackboard (AI|GetAIController self)) (Utilities|Name|MakeLiteralName "SeeingPlayer") false))))

(event EventBeginPlay
  (Utilities|Time|SetTimerbyEvent (delegate Custom|Stop%20SeeingPlayer) 0.5 true))

(fn ConstructionScript)
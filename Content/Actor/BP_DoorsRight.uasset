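; BP_DoorsRight is a key-locked interactable door that swings open and closed on a pivot.
; Interact toggles DoorsClosed and plays or reverses the OpenDoor timeline, which drives the yaw of the Pivto component.
; Pickupkey sets HasKey; without it, Interact only prints an Indonesian "no key" message.
; It always reports itself interactible and caches the player character on BeginPlay, though these graphs never use that reference.
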(event EventBeginPlay
  (bind _asbp_third_person_character (Utilities|Casting|CastToBP_ThirdPersonCharacter (Game|GetPlayerCharacter 0)))
  (Variables|Default|SetCharacter _asbp_third_person_character))

(event Collision|EventActorBeginOverlap
  (params (OtherActor :type Actor%20Object%20Reference)))

(event EventTick
  (params (DeltaSeconds :type Float%20%28single-precision%29)))

(event EventInteract
  (params (MyActor :type BP%20Third%20Person%20Character%20Object%20Reference))
  (bind _pivto (Variables|Default|GetPivto))
  (bind _relativerotation (Variables|/Script/Engine.SceneComponent|GetRelativeRotation _pivto))
  (if (Variables|Default|GetHasKey?)
    (if (Variables|Default|GetDoorsClosed)
      (Variables|Default|SetDoorsClosed false)
      (bind _door (Timeline|OpenDoor Play)
        (:Update
          (Transformation|SetRelativeRotation _pivto (Math|Rotator|MakeRotator (.roll _relativerotation) (.pitch _relativerotation) _door) false false)))
      (else
        (Variables|Default|SetDoorsClosed true)
        (Timeline|OpenDoor Reverse)))
    (else
      (Development|PrintString "Gak ada kunci bang"))))

(event EventPickupkey
  (Variables|Default|SetHasKey? true))

(fn ConstructionScript)

(fn ISINTERACTIBLE
  (return true))
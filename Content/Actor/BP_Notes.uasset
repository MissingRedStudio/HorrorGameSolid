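; BP_Notes is an interactable note actor that the player can read.
; It caches the player's BP_ThirdPersonCharacter at BeginPlay and always reports itself as interactable.
; On Interact, it copies its note description to the character, shows the note widget through the character's master UI reference and flags the character as reading.
; Closing the note and clearing that flag are not handled here.
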(event EventBeginPlay
  (bind _asbp_third_person_character (Utilities|Casting|CastToBP_ThirdPersonCharacter (Game|GetPlayerCharacter 0)))
  (Variables|Default|SetCharacter _asbp_third_person_character))

(event Collision|EventActorBeginOverlap
  (params (OtherActor :type Actor%20Object%20Reference)))

(event EventTick
  (params (DeltaSeconds :type Float%20%28single-precision%29)))

(event EventInteract
  (params (MyActor :type BP%20Third%20Person%20Character%20Object%20Reference))
  (bind _character (Variables|Default|GetCharacter))
  (Variables|/Game/ThirdPerson/Blueprints/BP_ThirdPersonCharacter.BP_ThirdPersonCharacter_C|SetNote _character (Variables|Default|GetNoteDescriptein))
  (Widget|SetVisibility (Variables|/Game/UI/WB_MasterUI.WB_MasterUI_C|GetWB_Note (Variables|/Game/ThirdPerson/Blueprints/BP_ThirdPersonCharacter.BP_ThirdPersonCharacter_C|GetMaster%20ui%20ref _character)) "Visible")
  (Variables|/Game/ThirdPerson/Blueprints/BP_ThirdPersonCharacter.BP_ThirdPersonCharacter_C|SetIsReading? (Variables|Default|GetCharacter) true))

(fn ConstructionScript)

(fn ISINTERACTIBLE
  (return true))
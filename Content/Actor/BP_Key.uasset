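; BP_Key is an interactable key pickup actor that notifies two referenced doors when the player collects it.
; It reports itself as interactible, and Interact calls Pickupkey on both doors, plays a key pickup sound and destroys the key.
; BeginPlay caches the player as a BP_ThirdPersonCharacter, though the reference is not used afterward, and its own Pickupkey event is empty.
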(event EventBeginPlay
  (bind _asbp_third_person_character (Utilities|Casting|CastToBP_ThirdPersonCharacter (Game|GetPlayerCharacter 0)))
  (Variables|Default|SetCharacter _asbp_third_person_character))

(event Collision|EventActorBeginOverlap
  (params (OtherActor :type Actor%20Object%20Reference)))

(event EventTick
  (params (DeltaSeconds :type Float%20%28single-precision%29)))

(event EventInteract
  (params (MyActor :type BP%20Third%20Person%20Character%20Object%20Reference))
  (Default|Pickupkey (Variables|Default|GetDoor))
  (Audio|PlaySound2D "/Game/Audio/086055_keys-pickupwav-39923.086055_keys-pickupwav-39923" 1.0 1.0 0.0 0 0)
  (Actor|DestroyActor))

(event EventPickupkey)

(fn ConstructionScript)

(fn ISINTERACTIBLE
  (return true))
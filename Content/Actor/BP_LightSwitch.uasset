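; Wall-switch style interactable actor that turns a referenced light on and off when the player interacts with it.
; Interact checks that the Light is valid, plays a switch sound and flips the light component's visibility.
; The LightSwticer timeline plays when switching on and reverses when switching off, sliding the Trigger component along relative X.
; It always reports itself interactible and caches the player character on BeginPlay.
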(event EventBeginPlay
  (bind _asbp_third_person_character (Utilities|Casting|CastToBP_ThirdPersonCharacter (Game|GetPlayerCharacter 0)))
  (Variables|Default|SetCharacter _asbp_third_person_character))

(event Collision|EventActorBeginOverlap
  (params (OtherActor :type Actor%20Object%20Reference)))

(event EventTick
  (params (DeltaSeconds :type Float%20%28single-precision%29)))

(event EventInteract
  (params (MyActor :type BP%20Third%20Person%20Character%20Object%20Reference))
  (bind _light (Variables|Default|GetLight))
  (bind _trigger (Variables|Default|GetTrigger))
  (bind _lightcomponent (Variables|/Script/Engine.Light|GetLightComponent _light))
  (bind _relativelocation (Variables|/Script/Engine.SceneComponent|GetRelativeLocation _trigger))
  (Utilities|IsValid _light
    (:Is%20Valid
      (if (Variables|/Script/Engine.SceneComponent|GetbVisible _lightcomponent)
        (Audio|PlaySound2D "/Game/Audio/FlashlightSwitch.FlashlightSwitch" 1.0 1.0 0.0 0 0)
        (Rendering|SetVisibility _lightcomponent false false)
        (bind _alpha (Timeline|Light%20Swticer Reverse)
          (:Update
            (Transformation|SetRelativeLocation _trigger (Math|Vector|MakeVector _alpha (.y _relativelocation) (.z _relativelocation)) false false)))
        (else
          (Audio|PlaySound2D "/Game/Audio/FlashlightSwitch.FlashlightSwitch" 1.0 1.0 0.0 0 0)
          (Rendering|SetVisibility _lightcomponent true false)
          (Timeline|Light%20Swticer Play))))))

(fn ConstructionScript)

(fn NewFunction
  (params (self2 :type Scene%20Component%20Object%20Reference)))

(fn ISINTERACTIBLE
  (return true))